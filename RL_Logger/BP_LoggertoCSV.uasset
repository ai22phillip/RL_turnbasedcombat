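; BP_LoggertoCSV records per-episode game statistics to CSV, apparently for reinforcement learning given its RL_Logger folder and reward field.
; SaveDataToCSV passes turns, attacks, movement, win flag, enemy and player health, and rewards to AppendRowToCSV.
; It then resets all those variables to zero or false for the next record.
; The counters are not updated within this graph, and BeginPlay is empty.
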(event Custom|SaveDataToCSV
  (Class|BPLoggertoCSV|AppendRowtoCSV (Variables|Default|GetTurns) (Variables|Default|GetAttacks) (Variables|Default|GetMovement) (Variables|Default|GetWon) (Variables|Default|GetEnemy%20Health) (Variables|Default|GetPlayer%20Health) (Variables|Default|GetRewards))
  (Utilities|FlowControl|Sequence
    (:then_0
      (Variables|Default|SetWon false))
    (:then_1
      (Variables|Default|SetRewards 0.0))
    (:then_2
      (Variables|Default|SetEnemy%20Health 0))
    (:then_3
      (Variables|Default|SetPlayer%20Health 0))
    (:then_4
      (Variables|Default|SetMovement 0))
    (:then_5
      (Variables|Default|SetTurns 0))
    (:then_6
      (Variables|Default|SetAttacks 0))))

(event EventBeginPlay)

(event Collision|EventActorBeginOverlap
  (params (OtherActor :type Actor%20Object%20Reference)))

(event EventTick
  (params (DeltaSeconds :type Float%20%28single-precision%29)))

(fn ConstructionScript)